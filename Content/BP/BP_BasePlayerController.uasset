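; Base player controller that manages the on-screen display of selected units.
; On BeginPlay it sets Game and UI input with the mouse always locked and creates a UnitAreaWidget, caching its UnitBox.
; SetActiveUnit casts the unit to BP_BaseUnitCharacter and adds that unit's own SelectedUnitWidget to the box.
; SetDeactiveUnit takes no unit and removes the box's first child, and both events print debug strings.
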(event `self.ReceiveBeginPlay`
  (`WidgetBlueprintLibrary.SetInputMode_GameAndUIEx` self null "LockAlways")
  (bind _returnvalue (`|CreateWidget` "/Game/UI/WidgetUnit/UnitAreaWidget.UnitAreaWidget_C"))
  (bind _output_get (set `self.UnitAreaWidget` _returnvalue))
  (`UserWidget.AddToViewport` _output_get 0)
  (set `self.Unit Box` (`/Game/UI/WidgetUnit/UnitAreaWidget.UnitBox` _output_get)))

(event `self.SetActiveUnit`
  (params (ActUnit :type "BaseUnitCharacter Object Reference") (isActive :type Boolean))
  (`KismetSystemLibrary.PrintString` "Active" true true (struct :`R` 1.0 :`G` 0.06707 :`A` 1.0))
  (bind _asbp_base_unit_character (cast `/Game/BP/BP_BaseUnitCharacter` ActUnit))
  (bind _output_get (set `self.UnitSelectedWidget` (`/Game/BP/BP_BaseUnitCharacter.SelectedUnitWidget` _asbp_base_unit_character)))
  (`HorizontalBox.AddChildToHorizontalBox` (`/Game/UI/WidgetUnit/UnitAreaWidget.UnitBox` (stale `self.ReceiveBeginPlay` _output_get)) _output_get))

(event `self.SetDeactiveUnit`
  (`KismetSystemLibrary.PrintString` "Deactive" true true (struct :`R` 1.0 :`G` 0.06707 :`A` 1.0))
  (`PanelWidget.RemoveChildAt` (`self.Unit Box`) 0))

(fn `UserConstructionScript`)