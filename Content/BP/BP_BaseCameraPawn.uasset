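; BP_BaseCameraPawn is a camera pawn that zooms by moving itself vertically with the mouse wheel.
; Wheel up lowers the pawn while it is above a minimum height, and wheel down raises it while below a maximum.
; Each step is a world Z offset scaled by current height and delta seconds, so steps grow with altitude.
; Tick, overlap and construction script are empty.
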(event `Key|MouseScrollUp`
  (params (Key :type "Key Structure"))
  (bind (_returnvalue_x _returnvalue_y _returnvalue_z) (`KismetMathLibrary.BreakVector` (`self.K2_GetActorLocation` self)))
  (:`Pressed`
    (if (> _returnvalue_z 500.0)
      (bind (_returnvalue_x_2 _returnvalue_y_2 _returnvalue_z_2) (`KismetMathLibrary.BreakVector` (* (+ _returnvalue_z (0.0 0.0 1.0)) (stale `self.ReceiveTick` DeltaSeconds))))
      (`self.K2_AddActorWorldOffset` (`KismetMathLibrary.MakeVector` 0.0 0.0 (* _returnvalue_z_2 -2.0))))))

(event `self.ReceiveTick`
  (params (DeltaSeconds :type "Float (single-precision)")))

(event `Key|MouseScrollDown`
  (params (Key :type "Key Structure"))
  (bind (_returnvalue_x _returnvalue_y _returnvalue_z) (`KismetMathLibrary.BreakVector` (`self.K2_GetActorLocation` self)))
  (:`Pressed`
    (if (< _returnvalue_z 1000.0)
      (bind (_returnvalue_x_2 _returnvalue_y_2 _returnvalue_z_2) (`KismetMathLibrary.BreakVector` (* (+ _returnvalue_z (0.0 0.0 -1.0)) (stale `self.ReceiveTick` DeltaSeconds))))
      (`self.K2_AddActorWorldOffset` (`KismetMathLibrary.MakeVector` 0.0 0.0 (* _returnvalue_z_2 2.0))))))

(fn `UserConstructionScript`)