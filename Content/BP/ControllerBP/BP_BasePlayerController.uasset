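; Base player controller that builds the on-screen UI for unit selection and building.
; On BeginPlay it creates the unit area widget, nests the building widget in its build overlay, and adds a separate debug widget to the viewport.
; SetActiveUnit places the unit's own widget in the info overlay, and SetDeactiveUnit removes that overlay's first child.
; AddVertBoxElement is an empty stub, and the input-mode call is unconnected.
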(event `self.ReceiveBeginPlay`
  (bind _returnvalue (`|CreateWidget` "/Game/UI/BaseWidget/UnitAreaWidget.UnitAreaWidget_C"))
  (bind _output_get (set `self.UnitAreaWidget` _returnvalue))
  (`UserWidget.AddToViewport` _output_get 0)
  (bind _returnvalue_2 (`|CreateWidget` "/Game/UI/BuildingWidget/BP_BuildingWidget.BP_BuildingWidget_C"))
  (`Overlay.AddChildToOverlay` (`/Game/UI/BaseWidget/UnitAreaWidget.OverlayBuild` (`self.UnitAreaWidget`)) _returnvalue_2)
  (bind _returnvalue_3 (`|CreateWidget` "/Game/UI/DebugWidget/DebugWidget.DebugWidget_C"))
  (`UserWidget.AddToViewport` _returnvalue_3 0))

(event `self.SetActiveUnit`
  (params (ActUnit :type "BaseUnitCharacter Object Reference"))
  (`Overlay.AddChildToOverlay` (`/Game/UI/BaseWidget/UnitAreaWidget.OverlayInfo` (`self.UnitAreaWidget`)) (`BaseUnitCharacter.BaseUserWidget` ActUnit)))

(event `self.AddVertBoxElement`
  (params (UserWidget :type "BuildingWidget Object Reference")))

(event `self.SetDeactiveUnit`
  (`PanelWidget.RemoveChildAt` (`/Game/UI/BaseWidget/UnitAreaWidget.OverlayInfo` (`self.UnitAreaWidget`)) 0))

(fn `UserConstructionScript`)